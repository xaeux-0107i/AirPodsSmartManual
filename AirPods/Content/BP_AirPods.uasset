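; BP_AirPods is an AirPods actor that animates its rotation through two steps.
; The ZRotation timeline turns yaw from 180 to zero for step one, and a second timeline pitches it to -90 for step two.
; Each step's Start event plays its timeline, while Back first snaps to that step's starting rotation and replays forward.
; Reset restores the initial half-turn yaw.
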(event `Step1Back`
  (`self.K2_SetActorRotation` (`KismetMathLibrary.MakeRotator` 0.0 0.0 180.0))
  (bind (_direction _newtrack_0) (`Timeline|ZRotation` :!via `PlayFromStart` :!label _label)
    (:`Update`
      (`self.K2_SetActorRotation` (`KismetMathLibrary.MakeRotator` 0.0 0.0 (`KismetMathLibrary.Lerp` 180.0 0.0 _newtrack_0))))))

(event `Step1Start`
  (goto _label :!via `PlayFromStart`))

(event `Step2Back`
  (`self.K2_SetActorRotation` (`KismetMathLibrary.MakeRotator` 0.0 0.0 0.0))
  (bind (_direction _newtrack_0) (`Timeline|Timeline` :!via `PlayFromStart` :!label _label_2)
    (:`Update`
      (`self.K2_SetActorRotation` (`KismetMathLibrary.MakeRotator` 0.0 (`KismetMathLibrary.Lerp` 0.0 -90.0 _newtrack_0) 0.0)))))

(event `Step2Start`
  (goto _label_2 :!via `PlayFromStart`))

(event `Reset`
  (`self.K2_SetActorRotation` (`KismetMathLibrary.MakeRotator` 0.0 0.0 180.0)))

(fn `UserConstructionScript`)