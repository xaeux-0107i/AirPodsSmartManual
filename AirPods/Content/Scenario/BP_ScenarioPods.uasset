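; Interactive wireless earbud case that demonstrates opening, removing the pods, playback, volume and pairing.
; Left-mouse dragging spins the actor, while clicking LidBox toggles the lid, which gates the timeline-animated lifting of the pods.
; Hit areas on each pod toggle BGM and step its volume; holding PairingBox runs a timer that pings and hides PairingEffect.
; Tick lights LIGHT once pods are taken, and Charging/NotCharging events animate the Charger.
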(event `self.ReceiveBeginPlay`
  (`self.EnableInput` (`GameplayStatics.GetPlayerController` 0))
  (set `self.Pods Base Location` (`SceneComponent.RelativeLocation` (`self.Pods`)))
  (bind _output_get (set `self.volume` 0.5))
  (`AudioComponent.SetVolumeMultiplier` (`self.BGM`) _output_get)
  (`SceneComponent.SetVisibility` (`self.charger`) false false))

(event `self.ReceiveTick`
  (params (DeltaSeconds :type "Float (single-precision)"))
  (bind _light (`self.LIGHT`))
  (set `self.time` (+ (`self.time`) 1.0))
  (`|ExecutionSequence`
    (:`then_0`
      (if (`self.bIsDragging`)
        (bind _output_get (set `self.Current Mouse X` (`PlayerController.GetMousePosition` (`GameplayStatics.GetPlayerController` 0))))
        (`self.K2_AddActorLocalRotation` (`KismetMathLibrary.MakeRotator` 0.0 0.0 (* (- (`self.Last Mouse X`) _output_get) 0.01)))))
    (:`then_1`
      (if (`self.bIsTaken`)
        (`SceneComponent.SetVisibility` _light true false)
        (`PrimitiveComponent.SetMaterial` _light 0 "/Game/hand2/eliMT2.eliMT2")))))

(event `self.LidBox.OnClicked`
  (params (TouchedComponent :type "PrimitiveComponent Object Reference") (ButtonPressed :type "Key Structure"))
  (if (`self.bIsLidOpened`)
    (set `self.bIsLidOpened` false)
    (bind (_direction _openlid) (`Timeline|Timeline` :!via `PlayFromStart`)
      (:`Update`
        (`SceneComponent.K2_SetRelativeRotation` (`self.Lid`) (`KismetMathLibrary.MakeRotator` (`KismetMathLibrary.Lerp` -35.0 55.0 _openlid)) false false)))
    (else
      (set `self.bIsLidOpened` true)
      (bind (_direction_2 _openlid_2) (`Timeline|OpenLid` :!via `PlayFromStart`)
        (:`Update`
          (`SceneComponent.K2_SetRelativeRotation` (`self.Lid`) (`KismetMathLibrary.MakeRotator` (`KismetMathLibrary.Lerp` 55.0 -35.0 _openlid_2)) false false))))))

(event `Key|LeftMouseButton`
  (params (Key :type "Key Structure"))
  (:`Pressed`
    (set `self.bIsDragging` true)
    (set `self.Last Mouse X` (`PlayerController.GetMousePosition` (`GameplayStatics.GetPlayerController` 0))))
  (:`Released`
    (set `self.bIsDragging` false)))

(event `self.RightTop.OnClicked`
  (params (TouchedComponent :type "PrimitiveComponent Object Reference") (ButtonPressed :type "Key Structure"))
  (bind (_pods_base_location_x _pods_base_location_y _pods_base_location_z) (`KismetMathLibrary.BreakVector` (`self.Pods Base Location`)))
  (bind (_pods_base_location_x_2 _pods_base_location_y_2 _pods_base_location_z_2) (`KismetMathLibrary.BreakVector` (`self.Pods Base Location`)))
  (if (`self.bIsLidOpened`) :!label _label
    (if (`self.bIsTaken`)
      (set `self.bIsTaken` false)
      (bind (_direction _takeout) (`Timeline|Timeline_0` :!via `PlayFromStart`)
        (:`Update`
          (`SceneComponent.K2_SetRelativeLocation` (`self.Pods`) (`KismetMathLibrary.MakeVector` 0.0 0.0 (`KismetMathLibrary.Lerp` (+ _pods_base_location_z_2 20.0) _pods_base_location_z_2 _takeout)) false false)))
      (else
        (set `self.bIsTaken` true)
        (bind (_direction_2 _takeout_2) (`Timeline|Timeline_1` :!via `PlayFromStart`)
          (:`Update`
            (`SceneComponent.K2_SetRelativeLocation` (`self.Pods`) (`KismetMathLibrary.MakeVector` 0.0 0.0 (`KismetMathLibrary.Lerp` _pods_base_location_z (+ _pods_base_location_z 20.0) _takeout_2)) false false)))))))

(event `self.LeftTop.OnClicked`
  (params (TouchedComponent :type "PrimitiveComponent Object Reference") (ButtonPressed :type "Key Structure"))
  (goto _label))

(event `self.RightMid.OnReleased`
  (params (TouchedComponent :type "PrimitiveComponent Object Reference") (ButtonReleased :type "Key Structure"))
  (bind _bgm (`self.BGM`))
  (if (`self.bIsPlaying`) :!label _label_2
    (set `self.bIsPlaying` false)
    (`AudioComponent.Stop` _bgm)
    (else
      (set `self.bIsPlaying` true)
      (`AudioComponent.Play` _bgm 0.0))))

(event `self.LeftMid.OnReleased`
  (params (TouchedComponent :type "PrimitiveComponent Object Reference") (ButtonReleased :type "Key Structure"))
  (goto _label_2))

(event `self.LeftUp.OnReleased`
  (params (TouchedComponent :type "PrimitiveComponent Object Reference") (ButtonReleased :type "Key Structure"))
  (bind _output_get (set `self.volume` (`KismetMathLibrary.FClamp` (+ (`self.volume`) 0.1)) :!label _label_3))
  (`AudioComponent.SetVolumeMultiplier` (`self.BGM`) _output_get))

(event `self.RightUp.OnReleased`
  (params (TouchedComponent :type "PrimitiveComponent Object Reference") (ButtonReleased :type "Key Structure"))
  (goto _label_3))

(event `self.RightDown.OnReleased`
  (params (TouchedComponent :type "PrimitiveComponent Object Reference") (ButtonReleased :type "Key Structure"))
  (bind _output_get (set `self.volume` (`KismetMathLibrary.FClamp` (- (`self.volume`) 0.1)) :!label _label_4))
  (`AudioComponent.SetVolumeMultiplier` (`self.BGM`) _output_get))

(event `self.LeftDown.OnReleased`
  (params (TouchedComponent :type "PrimitiveComponent Object Reference") (ButtonReleased :type "Key Structure"))
  (goto _label_4))

(event `Charging`
  (set `self.bIsCharging` true)
  (`SceneComponent.SetVisibility` (`self.charger`) true false)
  (bind (_direction _newtrack_0) (`Timeline|Timeline_2` :!via `PlayFromStart`)
    (:`Update`
      (`SceneComponent.K2_SetRelativeLocation` (`self.charger`) (`KismetMathLibrary.MakeVector` 0.0 0.0 (+ (`KismetMathLibrary.Lerp` 0.0 25.0 _newtrack_0) -40.0)) false false))))

(event `NotCharging`
  (set `self.bIsCharging` false)
  (bind (_direction _newtrack_0) (`Timeline|Timeline_3` :!via `PlayFromStart`)
    (:`Update`
      (`SceneComponent.K2_SetRelativeLocation` (`self.charger`) (`KismetMathLibrary.MakeVector` 0.0 0.0 (+ (`KismetMathLibrary.Lerp` 0.0 -25.0 _newtrack_0) -15.0)) false false))
    (:`Finished`
      (`SceneComponent.SetVisibility` (`self.charger`) false false))))

(event `self.LidBox.OnBeginCursorOver`
  (params (TouchedComponent :type "PrimitiveComponent Object Reference"))
  (set `self.isLidHang` true))

(event `self.LidBox.OnEndCursorOver`
  (params (TouchedComponent :type "PrimitiveComponent Object Reference"))
  (set `self.isLidHang` false))

(event `self.PairingBox.OnClicked`
  (params (TouchedComponent :type "PrimitiveComponent Object Reference") (ButtonPressed :type "Key Structure"))
  (bind _returnvalue (`KismetSystemLibrary.K2_SetTimerDelegate` (delegate `Pairing`) 5.0)))

(event `self.PairingBox.OnReleased`
  (params (TouchedComponent :type "PrimitiveComponent Object Reference") (ButtonReleased :type "Key Structure"))
  (`KismetSystemLibrary.K2_ClearAndInvalidateTimerHandle` (stale `self.PairingBox.OnClicked` _returnvalue)))

(event `Pairing`
  (`GameplayStatics.PlaySound2D` "/Engine/EngineSounds/1kSineTonePing.1kSineTonePing" 1.0 1.0 0.0 null null)
  (`SceneComponent.SetVisibility` (`self.PairingEffect`) false false))

(fn `UserConstructionScript`)